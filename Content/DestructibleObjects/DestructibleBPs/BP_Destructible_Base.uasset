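; Base destructible object that loses one health per hit and breaks apart on death, printing the points awarded.
; OnHit spawns Niagara impact particles tinted from green to red by remaining health; once health is depleted, the next hit fires OnDeath once.
; ObjectExploded uses Chaos physics fields: radial strain at the mesh breaks clusters, and radial velocity from the hit location scatters the pieces.
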(event `OnDeath`
  (params (HitLocation :type "Vector Structure"))
  (`/Engine/EditorBlueprintResources/StandardMacros.DoOnce` false
    (:`Completed`
      (`self.Object Exploded` HitLocation)
      (`KismetSystemLibrary.PrintString` (`KismetTextLibrary.Conv_TextToString` (`|FormatText` "{0} Points Awarded" (`self.PointsAwarded`)))))))

(event `self.ReceiveBeginPlay`
  (set `self.CurrentHealth` (`KismetMathLibrary.Conv_IntToDouble` (`self.MaxHealth`))))

(fn `Object Exploded`
  (params (HitLocation :type "Vector Structure"))
  (bind _fieldsystem (`self.FieldSystem`))
  (`FieldSystemComponent.ApplyPhysicsField` _fieldsystem true "Field_ExternalClusterStrain" null (`RadialFalloff.SetRadialFalloff` (`self.RadialFalloff`) 500.0 0.0 1.0 0.0 100.0 (`SceneComponent.K2_GetComponentLocation` (`self.DestructibleMesh`)) "Field_FallOff_None"))
  (`FieldSystemComponent.ApplyPhysicsField` _fieldsystem true "Field_LinearVelocity" null (`RadialVector.SetRadialVector` (`self.RadialVector`) 700.0 (`local.HitLocation`))))

(fn `OnHit`
  (params (HitLocation :type "Vector Structure"))
  (if (<= (`self.CurrentHealth`) 0.0)
    (`/Engine/EditorBlueprintResources/StandardMacros.DoOnce` false
      (:`Completed`
        (`self.OnDeath` HitLocation)))
    (else
      (set `self.CurrentHealth` (- (`self.CurrentHealth`) 1.0))
      (`self.SpawnHitParticles` HitLocation))))

(fn `SpawnHitParticles`
  (params (HitLocation :type "Vector Structure"))
  (bind _returnvalue (`NiagaraFunctionLibrary.SpawnSystemAtLocation` "/Game/Particles/NS_HitImpact.NS_HitImpact" HitLocation))
  (`NiagaraComponent.SetVariableLinearColor` _returnvalue "ParticleColour" (`KismetMathLibrary.LinearColorLerp` (struct :`R` 1.0 :`B` 0.1 :`A` 1.0) (struct :`R` 0.5 :`G` 1.0 :`A` 1.0) (/ (`self.CurrentHealth`) (`self.MaxHealth`)))))

(fn `UserConstructionScript`)